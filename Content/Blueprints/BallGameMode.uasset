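; Game mode for a brick-and-paddle ball game that runs the match state machine, from ready and countdown through play to game over or completion.
; It counts bricks at start, completes the level when none remain, and opens the next numbered level via the game instance.
; SetGameState drives timed transitions, checking paddle lives after a miss and showing a play-again widget at the end.
; Tick runs the three-second countdown before calling StartPlaying.
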(event Custom|StartCountdown
  (Variables|Default|SetCountdown 3.0)
  (Variables|Default|SetStateOfTheGame "NewEnumerator1"))

(event Custom|SetGameState
  (params (StateOfGame :type StateOfGame%20Enum :default "NewEnumerator0"))
  (switch Utilities|FlowControl|Switch|SwitchonStateOfGame StateOfGame
    (:NewEnumerator0
      (Variables|Default|SetStateOfTheGame StateOfGame))
    (:NewEnumerator1
      (Variables|Default|SetCountdown 3.0)
      (Variables|Default|SetStateOfTheGame "NewEnumerator1"))
    (:NewEnumerator2
      (Variables|Default|SetStateOfTheGame "NewEnumerator2")
      (Utilities|FlowControl|Delay 0.75)
      (bind _aspaddle (Utilities|Casting|CastToPaddle (Game|Player|GetPlayerPawn 0)))
      (if (<= (Variables|/Game/Blueprints/Paddle.Paddle_C|GetLives _aspaddle) 0)
        (CallFunction|SetGameState "NewEnumerator3")
        (else
          (CallFunction|SetGameState "NewEnumerator0"))))
    (:NewEnumerator3
      (Variables|Default|SetStateOfTheGame "NewEnumerator3")
      (Utilities|FlowControl|Delay 1.0)
      (CallFunction|AskPlayAgain))
    (:NewEnumerator4
      (Variables|Default|SetStateOfTheGame "NewEnumerator4")
      (Utilities|FlowControl|Delay 1.5)
      (bind _asball_game_instance (Utilities|Casting|CastToBallGameInstance (Game|GetGameInstance)))
      (if (== (Variables|/Game/Blueprints/BallGameInstance.BallGameInstance_C|GetCurrentLevel _asball_game_instance) (Variables|/Game/Blueprints/BallGameInstance.BallGameInstance_C|GetMaxLevels _asball_game_instance))
        (CallFunction|SetGameState "NewEnumerator7")
        (else
          (bind _result (Math|Integer|IncrementInt (Variables|/Game/Blueprints/BallGameInstance.BallGameInstance_C|GetCurrentLevel _asball_game_instance))
            (:%20%20
              (Game|OpenLevel(byName) (Utilities|String|StringToName (Utilities|String|Append "Level" (Utilities|String|ToString(Integer) _result)))))))))
    (:NewEnumerator5
      (Default|CallStartPlaying)
      (Variables|Default|SetStateOfTheGame "NewEnumerator5"))
    (:NewEnumerator6
      (Variables|Default|SetStateOfTheGame "NewEnumerator6")
      (Game|SetGamePaused true))
    (:NewEnumerator7
      (Variables|Default|SetStateOfTheGame "NewEnumerator7")
      (Utilities|FlowControl|Delay 1.5)
      (CallFunction|AskPlayAgain))))

(event EventBeginPlay
  (Variables|Default|SetStateOfTheGame "NewEnumerator0")
  (bind _outactors (Actor|GetAllActorsOfClass "/Game/Blueprints/Brick.Brick_C"))
  (for _array_element _outactors
    (Math|Integer|IncrementInt (Variables|Default|GetBrickCount))))

(event EventTick
  (params (DeltaSeconds :type Float%20%28single-precision%29))
  (if (Utilities|Enum|Equal(Enum) (Variables|Default|GetStateOfTheGame) "NewEnumerator1")
    (bind _output_get (Variables|Default|SetCountdown (- (Variables|Default|GetCountdown) DeltaSeconds)))
    (if (>= _output_get 2.0)
      (Variables|Default|SetCount 3)
      (elif (>= (Variables|Default|GetCountdown) 1.0)
        (Variables|Default|SetCount 2)
        (elif (>= (Variables|Default|GetCountdown) 0.0)
          (Variables|Default|SetCount 1)
          (else
            (CallFunction|SetGameState "NewEnumerator5")))))))

(fn ConstructionScript)

(fn AskPlayAgain
  (bind _returnvalue (Game|GetPlayerController 0))
  (bind _returnvalue_2 (UserInterface|CreateWidget "/Game/HUD/PlayAgain.PlayAgain_C"))
  (bind _output_get (Variables|Default|SetAskWidget _returnvalue_2))
  (UserInterface|Viewport|AddtoViewport _output_get 0)
  (Variables|/Script/Engine.PlayerController|SetbShowMouseCursor _returnvalue true)
  (Input|SetInputModeUIOnly _returnvalue 0 "DoNotLock"))

(fn DecrementBrickCount
  (bind _result (Math|Integer|DecrementInt (Variables|Default|GetBrickCount))
    (:%20%20
      (if (<= _result 0)
        (CallFunction|SetGameState "NewEnumerator4")))))